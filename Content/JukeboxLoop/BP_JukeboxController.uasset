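; BP_JukeboxController is a mod controller that keeps the level's jukebox playing continuously.
; On BeginPlay it finds BP_JukeBox, async-loads the mod's enabled setting from a save slot and listens for the random cue's audio-finished event.
; When audio finishes or the setting is applied, it restarts an idle jukebox by simulating the player's Use on its InstantUsable, if enabled.
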(event `self.ReceiveBeginPlay`
  (bind _returnvalue (`GameplayStatics.GetActorOfClass` "/Game/Art/Environments/ShipTesting/BP_JukeBox.BP_JukeBox_C"))
  (set `self.Jukebox` _returnvalue)
  (`KismetSystemLibrary.Delay` 1.0)
  (`self.LoadAsync`)
  (bind _jukebox (`self.Jukebox`)
    (:`then`
      (add `AudioComponent.OnAudioFinished` (`/Game/Art/Environments/ShipTesting/BP_JukeBox.JukeBox_Random_Cue` _jukebox) (delegate `OnAudioFinished`)))
    (:`else`)))

(event `OnAudioFinished`
  (`KismetSystemLibrary.Delay` 0.2)
  (`self.TryEnableJukebox`))

(event `TryEnableJukebox`
  (if (`self.ModEnabled`)
    (bind _jukebox (`self.Jukebox`)
      (:`then`
        (bind _jukebox_random_cue (`/Game/Art/Environments/ShipTesting/BP_JukeBox.JukeBox_Random_Cue` _jukebox))
        (`/Engine/EditorBlueprintResources/StandardMacros.IsValid` _jukebox_random_cue
          (:`Is Valid`
            (if (not (`AudioComponent.IsPlaying` _jukebox_random_cue))
              (bind _asplayer_character (cast `PlayerCharacter` (`GameplayStatics.GetPlayerPawn` 0)))
              (`UsableComponentBase.BeginUse` (`/Game/Art/Environments/ShipTesting/BP_JukeBox.InstantUsable` _jukebox) _asplayer_character "Use")))))
      (:`else`))))

(event `LoadAsync`
  (bind _savegame (`AsyncActionHandleSaveGame.AsyncLoadGameFromSlot` (`/Game/JukeboxLoop/SaveSystem/BPFL_ModSaveSlots.GetSettingsSlot`))
    (:`Completed`
      (`|ExecutionSequence`
        (:`then_0`
          (bind _assg_mod_settings (cast `/Game/JukeboxLoop/SaveSystem/SG_ModSettings` _savegame))
          (`self.SetModEnabled` (`/Game/JukeboxLoop/SaveSystem/SG_ModSettings.ModEnabled` _assg_mod_settings)))
        (:`then_1`
          (set `self.Loaded` true)
          (`self.OnLoaded`))))))

(fn `SetModEnabled`
  (params (Enabled :type Boolean))
  (set `self.ModEnabled` Enabled)
  (`self.TryEnableJukebox`))

(fn `UserConstructionScript`)

(fn `WasLoaded`
  (returns (WasLoaded :type Boolean))
  (return (`self.Loaded`)))